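; BP_CombatUnit is a grid-based combat unit that animates successful and failed moves.
; A successful move gets the world position for its grid coordinate from BasicLevelGameModeEMP, then a double-speed timeline lerps the actor there.
; A failed move plays a separate timeline that lerps toward a short fixed offset along world X.
; Either animation can optionally notify the game mode when finished.
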(event `self.HandleMoveToLocation`
  (params (bNotifyWhenFinished :type Boolean))
  (bind _asbasic_level_game_mode_emp (cast `BasicLevelGameModeEMP` (`GameplayStatics.GetGameMode`)))
  (bind _returnvalue (`BasicLevelGameModeEMP.GetWorldLocationFromGridLocation` _asbasic_level_game_mode_emp (`self.GridCoordinate`)))
  (set `self.TargetLocation` _returnvalue)
  (set `self.StartingLocation` (`self.K2_GetActorLocation`))
  (`TimelineComponent.SetPlayRate` (`self.MoveToNewLocation`) 2.0)
  (bind (_direction _alpha) (`Timeline|MoveToNewLocation` :!via `PlayFromStart`)
    (:`Update`
      (`self.K2_SetActorLocation` (`KismetMathLibrary.VLerp` (`self.StartingLocation`) (`self.TargetLocation`) _alpha)))
    (:`Finished`
      (if bNotifyWhenFinished
        (`BasicLevelGameModeEMP.HandleCombatUnitAnimationFinished` _asbasic_level_game_mode_emp)))))

(event `self.HandleMovementFailed`
  (params (bNotifyWhenFinished :type Boolean))
  (bind _returnvalue (`self.K2_GetActorLocation`))
  (bind _asbasic_level_game_mode_emp (cast `BasicLevelGameModeEMP` (`GameplayStatics.GetGameMode`)))
  (set `self.StartingLocation` _returnvalue)
  (set `self.TargetLocation` (+ _returnvalue (40.0 0.0 0.0)))
  (`TimelineComponent.SetPlayRate` (`self.MovementFailed`) 2.0)
  (bind (_direction _alpha) (`Timeline|MovementFailed` :!via `PlayFromStart`)
    (:`Update`
      (`self.K2_SetActorLocation` (`KismetMathLibrary.VLerp` (`self.StartingLocation`) (`self.TargetLocation`) _alpha)))
    (:`Finished`
      (if bNotifyWhenFinished
        (`BasicLevelGameModeEMP.HandleCombatUnitAnimationFinished` _asbasic_level_game_mode_emp)))))

(fn `UserConstructionScript`)