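; Archer combat class that represents a ranged unit on a chess-piece mesh with an ally or enemy gradient material.
; On attack it stores the target, plays the bow shoot montage on the weapon and fires on the montage notify.
; Firing spawns a BP_Arrow raised above the actor's origin and launches it at the equally raised target with a short flight time and zero apex offset.
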(event `self.HandleSetBaseMaterial`
  (params (bIsFriendly :type Boolean))
  (`PrimitiveComponent.SetMaterial` (`self.Chess`) 0 (select `bool` bIsFriendly :`false` "/Game/Materials/Gradients/MI_EnemyGradient.MI_EnemyGradient" :`true` "/Game/Materials/Gradients/MI_AllyGradient.MI_AllyGradient" :!type "MaterialInterface Object Reference")))

(event `self.HandleAttackTriggered`
  (params (InTargetLocation :type "Vector Structure"))
  (set `self.TargetLocation` InTargetLocation)
  (`|PlayMontage` (`self.Weapon`) "/Game/Models/Chess/Bow/Bow_Animated_Root_Shoot_Montage.Bow_Animated_Root_Shoot_Montage"
    (:`OnNotifyBegin`
      (`self.LaunchArrow` 0.1 0.0 (`self.TargetLocation`)))))

(event `LaunchArrow`
  (params (FlightTime :type "Float (double-precision)") (DeltaApex :type "Float (double-precision)") (ArrowTarget :type "Vector Structure"))
  (bind (_returnvalue_x _returnvalue_y _returnvalue_z) (`KismetMathLibrary.BreakVector` (`self.K2_GetActorLocation`)))
  (bind _returnvalue (`|SpawnActorFromClass` "/Game/Combat/BP_Arrow.BP_Arrow_C" (`KismetMathLibrary.MakeTransform` (`KismetMathLibrary.MakeVector` _returnvalue_x _returnvalue_y (+ _returnvalue_z 60.0))) "Undefined" "OverrideRootScale" null null))
  (`/Game/Combat/BP_Arrow.LaunchArrow` _returnvalue (`KismetMathLibrary.MakeVector` (.x ArrowTarget) (.y ArrowTarget) (+ (.z ArrowTarget) 60.0)) FlightTime DeltaApex))

(fn `UserConstructionScript`)