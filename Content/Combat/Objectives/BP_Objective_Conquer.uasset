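; BP_Objective_Conquer is a combat objective that grants victory when every enemy squad is gone.
; On initialization it stores the combat game mode and binds to its squad-removed-from-combat event.
; Each removal runs a check that fires objective completion if at least one friendly squad remains and no enemy squads do.
; It also supplies objective text describing victory as breaking the opposing side or forcing it to retreat.
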(event `self.InitializeObjective`
  (params (CombatGameMode :type "EMPCombatMapGameMode Object Reference"))
  (bind _output_get (set `self.Combat Game Mode` CombatGameMode))
  (add `EMPCombatMapGameMode.OnSquadRemovedFromCombat` _output_get (delegate `OnSquadRemovedFromCombat_Event_0`)))

(event `OnSquadRemovedFromCombat_Event_0`
  (params (squadData :type "EMPSquadData Object Reference"))
  (`self.CheckWinCondition`))

(event `CheckWinCondition`
  (if (and (> (`EMPCombatMapGameMode.GetNumberOfFriendlySquads` (`self.Combat Game Mode`)) 0) (== (`EMPCombatMapGameMode.GetNumberOfEnemySquads` (`self.Combat Game Mode`)) 0))
    (`self.OnObjectiveComplete` self)))

(fn `GetObjectiveText`
  (returns (ReturnValue :type Text))
  (return "Victory when opposing side is completely broken or chooses to retreat."))