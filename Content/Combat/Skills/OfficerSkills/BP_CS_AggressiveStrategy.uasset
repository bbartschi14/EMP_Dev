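; BP_CS_AggressiveStrategy is an officer combat skill that alters attack damage while the owning squad follows an aggressive strategy.
; Only combat units of Lieutenant officer rank meet its requirements.
; ModifyDamage scales damage by DamageMultiplier and truncates it to an integer when the squad strategy is Aggressive and the action is an attack, otherwise returning the original value.
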(fn `AreSkillRequirementsMet`
  (params (Squad :type "EMPSquadData Object Reference") (CombatUnit :type "EMPCombatUnitData Object Reference"))
  (returns (ReturnValue :type Boolean))
  (return (`|EnumEquality` (`EMPCombatUnitData.OfficerRank` CombatUnit) "OR_LIEUTENANT")))

(fn `ModifyDamage`
  (params (OriginalDamage :type Integer))
  (returns (ReturnValue :type Integer))
  (bind (_data_owningunit _data_otherunit _data_bisattack) (break `EMPStatModifierCombatSkillData` (`self.Data`)))
  (return (`KismetMathLibrary.SelectInt` (`KismetMathLibrary.FTrunc` (* OriginalDamage (`self.DamageMultiplier`))) OriginalDamage (and (`|EnumEquality` (`EMPSquadData.GetSquadStrategy` (`EMPCombatUnitData.OwningSquad` _data_owningunit)) "AGGRESSIVE") _data_bisattack))))