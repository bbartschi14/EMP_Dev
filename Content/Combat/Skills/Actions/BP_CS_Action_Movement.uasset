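; Combat skill action that moves a squad one orthogonally adjacent grid area, available to all squads.
; Selecting a valid area stores the destination, spawns an arrow indicator and confirms the queued action.
; On execution, a macro checks occupancy: empty areas allow movement, same-side squads block it, and opposing squads initiate combat.
; Completion is signalled after a timed delay, or when the game mode's combat-simulation-finished event fires.
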(event `self.OnExecuteAction`
  (bind _owninggamemode (`self.OwningGameMode`))
  (bind _owninggamemode_2 (`self.OwningGameMode`))
  ;[1 0.6459 0.09166] Primary Overrides
  (bind (_friendlycombatsquad _enemycombatsquad) (`self.SwitchOnMovementResult`)
    (:`Can Move`
      (`EMPCombatMapGameMode.MoveSquadToAreaLocation` _owninggamemode_2 (`self.OwningSquad`) (`self.DestinationCoord`) 0.75)
      (`EMPBPFunctionLibrary.DelayWorld` _owninggamemode_2 0.75)
      (`self.OnExecutionFinished`) ; Must call this function to indicate finished!
    )
    (:`Can't Move`
      (`EMPCombatMapGameMode.HandleSquadMovementFailed` _owninggamemode_2 (`self.OwningSquad`) 0.5)
      (`EMPBPFunctionLibrary.DelayWorld` _owninggamemode_2 0.5)
      (`self.OnExecutionFinished`) ; Must call this function to indicate finished!
    )
    (:`Combat Will Initiate`
      (add `EMPCombatMapGameMode.OnCombatSimuationFinished` _owninggamemode (delegate `OnCombatSimuationFinished_Event_0`))
      (`EMPCombatMapGameMode.InitiateCombat` _owninggamemode _friendlycombatsquad _enemycombatsquad))))

(event `OnCombatSimuationFinished_Event_0`
  ;[1 0.6459 0.09166] Primary Overrides
  (remove `EMPCombatMapGameMode.OnCombatSimuationFinished` (`self.OwningGameMode`) (delegate `OnCombatSimuationFinished_Event_0`))
  (`self.OnExecutionFinished`) ; Must call this function to indicate finished!
)

(event `self.HandleGridSelected`
  (params (InGridCoordinate :type "IntPoint Structure") (InGridArea :type "IntPoint Structure"))
  ;[1 0.6459 0.09166] Primary Overrides
  (bind _canmove (`self.CanSquadMoveToCoord` InGridArea))
  (if _canmove
    (bind _output_get (set `self.DestinationCoord` InGridArea))
    (`EMPCombatMapGrid.SpawnArrowIndicator` (`EMPCombatMapGameMode.Grid` (`self.OwningGameMode`)) self (`EMPSquadData.CombatAreaLocation` (`self.OwningSquad`)) _output_get)
    (`self.ConfirmQueue`) ; Call this when ready to stop waiting for input
  ))

(fn `AreSkillRequirementsMet`
  (params (Squad :type "EMPSquadData Object Reference") (CombatUnit :type "EMPCombatUnitData Object Reference"))
  (returns (ReturnValue :type Boolean))
  ;[1 1 1] Valid for all squads
  (return true))

(fn `CanSquadMoveToCoord`
  (params (DesiredCoord :type "IntPoint Structure"))
  (returns (CanMove :type Boolean))
  (bind (_returnvalue_x _returnvalue_y) (break `IntPoint` (- (`EMPSquadData.CombatAreaLocation` (`self.OwningSquad`)) DesiredCoord)))
  (return (== (+ (`KismetMathLibrary.Abs_Int` _returnvalue_x) (`KismetMathLibrary.Abs_Int` _returnvalue_y)) 1)))

(fn `GetQueuedActionText`
  (returns (ReturnValue :type Text))
  (return (`|FormatText` "{squadName} moving to area {destination}" (`EMPSquadData.SquadName` (`self.OwningSquad`)) (`KismetStringLibrary.Conv_IntPointToString` (`self.DestinationCoord`)))))

(fn `IsGridAreaSelectable`
  (params (InGridArea :type "IntPoint Structure"))
  (returns (ReturnValue :type Boolean))
  (bind _canmove (`self.CanSquadMoveToCoord` InGridArea))
  (return _canmove))

(fn `IsGridCoordinateSelectable`
  (params (InGridCoordinate :type "IntPoint Structure"))
  (returns (ReturnValue :type Boolean))
  (return false))