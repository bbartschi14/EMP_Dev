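; Combat skill action that lets a squad with archers fire repeated arrow volleys at a grid area within Manhattan range.
; Selecting an area spawns an arrow indicator and confirms the queued action.
; On execution, each archer arcs an arrow at a random sub-space per volley, recording hits on enemies there immediately.
; A parallel delayed loop pops and resolves those hits as arrows land, finishing after the last volley.
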(event `ShootArrowAtLocation`
  (params (ArcherUnit :type "EMPCombatUnitData Object Reference") (gridLocation :type "IntPoint Structure"))
  (bind _asbp_combat_unit (cast `/Game/Combat/BP_CombatUnit` (`EMPCombatUnitData.CombatUnitActor` ArcherUnit)))
  (bind _asbp_combat_class_archer (cast `/Game/Combat/Classes/BP_CombatClass_Archer` (`/Game/Combat/BP_CombatUnit.CombatClassActor` _asbp_combat_unit)))
  (`/Game/Combat/Classes/BP_CombatClass_Archer.LaunchArrow` _asbp_combat_class_archer 2.0 1000.0 (`EMPGrid.GetWorldLocationFromGridLocation` (`EMPCombatMapGameMode.Grid` (`self.OwningGameMode`)) gridLocation)))

(event `self.OnExecuteAction`
  ;[1 1 1] Action Execution
  (set `self.NumberOfCompletedVolleys` 0)
  (`|ExecutionSequence`
    (:`then_0`
      (`/Game/Combat/Skills/Actions/Macros_CS_Actions.ForLoopWithDelay` 0 (- (`self.NumVolleys`) 1) 0.5
        (:`LoopBody`
          (bind _hits (`self.ShootVolley`))
          (`KismetArrayLibrary.Array_Add` (`self.VolleyHitResults`) _hits))))
    (:`then_1`
      ;;[0 0 0] Due to the way that delay nodes queue execution, this delay node will trigger at the same time that the "Then 0" branch of the sequence node starts. Thus we wait for the amount of time that it will take for the first volley to hit before starting the pop loop
      (`EMPBPFunctionLibrary.DelayWorld` (`self.OwningGameMode`) 2.0)
      (`/Game/Combat/Skills/Actions/Macros_CS_Actions.ForLoopWithDelay` 0 (- (`self.NumVolleys`) 1) 0.5
        (:`LoopBody`
          (`self.PopAndResolveHits`))))))

(event `OnVolleyResolved`
  ;[1 1 1] Action Execution
  (bind _result (`/Engine/EditorBlueprintResources/StandardMacros.IncrementInt` (`self.NumberOfCompletedVolleys`))
    (:`  `
      (if (>= _result (`self.NumVolleys`))
        (`EMPBPFunctionLibrary.DelayWorld` (`self.OwningGameMode`) 0.5) ; Pause for just a moment
        (`self.OnExecutionFinished`) ; Must call this function to indicate finished!
      ))))

(event `self.HandleGridSelected`
  (params (InGridCoordinate :type "IntPoint Structure") (InGridArea :type "IntPoint Structure"))
  (bind _canvolley (`self.CanSquadVolleyToCoord` InGridArea))
  (if _canvolley
    (bind _output_get (set `self.DestinationCoord` InGridArea))
    (`EMPCombatMapGrid.SpawnArrowIndicator` (`EMPCombatMapGameMode.Grid` (`self.OwningGameMode`)) self (`EMPSquadData.CombatAreaLocation` (`self.OwningSquad`)) _output_get)
    (`self.ConfirmQueue`) ; Call this when ready to stop waiting for input
  ))

(fn `AreSkillRequirementsMet`
  (params (Squad :type "EMPSquadData Object Reference") (CombatUnit :type "EMPCombatUnitData Object Reference"))
  (returns (ReturnValue :type Boolean))
  ;[1 1 1] Valid for all squads
  (return (> (`EMPSquadData.GetNumberOfCombatUnitsOfClass` Squad "CC_ARCHER") 0)))

(fn `CanSquadVolleyToCoord`
  (params (DesiredCoord :type "IntPoint Structure"))
  (returns (CanVolley :type Boolean))
  (bind (_returnvalue_x _returnvalue_y) (break `IntPoint` (- (`EMPSquadData.CombatAreaLocation` (`self.OwningSquad`)) DesiredCoord)))
  (bind _returnvalue (+ (`KismetMathLibrary.Abs_Int` _returnvalue_x) (`KismetMathLibrary.Abs_Int` _returnvalue_y)))
  (return (and (<= _returnvalue (`self.VolleyDistance`)) (> _returnvalue 0))))

(fn `GetQueuedActionText`
  (returns (ReturnValue :type Text))
  (return (`|FormatText` "{squadName} volleying to area {destination}" (`EMPSquadData.SquadName` (`self.OwningSquad`)) (`KismetStringLibrary.Conv_IntPointToString` (`self.DestinationCoord`)))))

(fn `IsGridAreaSelectable`
  (params (InGridArea :type "IntPoint Structure"))
  (returns (ReturnValue :type Boolean))
  (bind _canvolley (`self.CanSquadVolleyToCoord` InGridArea))
  (return _canvolley))

(fn `IsGridCoordinateSelectable`
  (params (InGridCoordinate :type "IntPoint Structure"))
  (returns (ReturnValue :type Boolean))
  (return false))

(fn `PopAndResolveHits`
  (locals (LocalHits :type "EMPCombatHitResults Structure"))
  (bind _volleyhitresults (`self.VolleyHitResults`))
  (if (`KismetArrayLibrary.Array_IsValidIndex` (`self.VolleyHitResults`))
    (bind _output_get (set `local.LocalHits` (`|GetArrayItem` _volleyhitresults)))
    (`KismetArrayLibrary.Array_Remove` _volleyhitresults)
    (for _array_element (`.HitResults` (break `EMPCombatHitResults` _output_get))
      (`EMPCombatMapGameMode.ResolveHit` (`self.OwningGameMode`) _array_element))
    (`self.OnVolleyResolved`)))

(fn `ShootVolley`
  (returns (Hits :type "EMPCombatHitResults Structure"))
  (locals (VolleyHits :type "EMPCombatHitResults Structure"))
  (bind _volleyhits_hitresults (break `EMPCombatHitResults` (`local.VolleyHits`)))
  (bind _volleyhits_hitresults_2 (break `EMPCombatHitResults` (`local.VolleyHits`)))
  (`KismetArrayLibrary.Array_Clear` _volleyhits_hitresults_2)
  (for _array_element (`EMPSquadData.GetCombatUnitsOfClass` (`self.OwningSquad`) "CC_ARCHER")
    (bind _output_get (set `self.RandomCoord` (`self.RandomSubSpaceInArea` (`self.DestinationCoord`))))
    (`self.ShootArrowAtLocation` _array_element _output_get)
    (bind _enemyunit (`/Game/Combat/Skills/Actions/Macros_CS_Actions.FindEnemyUnitAtLocation` _output_get) ; Helper macro. Double click on node to see expanded logic
      (:`Exists`
        (`KismetArrayLibrary.Array_Add` _volleyhits_hitresults (make `EMPCombatHitResult` _array_element _enemyunit true (`EMPCombatUnitData.Damage` _array_element))))))
  (return (`local.VolleyHits`)))