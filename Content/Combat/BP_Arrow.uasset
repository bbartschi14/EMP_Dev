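; Arrow projectile actor that flies a scripted arc toward a target location over a given flight time, then destroys itself.
; LaunchArrow stores the endpoints and scales the MoveArrow timeline's play rate to the flight time.
; The timeline lerps XY and scales height by DeltaApex from the start Z, ignoring target Z and collision sweeps.
; Each update aims the mesh along its movement, with a -90 pitch offset.
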(event `LaunchArrow`
  (params (TargetLocation :type "Vector Structure") (FlightTime :type "Float (double-precision)") (DeltaApex :type "Float (double-precision)"))
  (bind _startinglocation (`self.StartingLocation`))
  (bind (_returnvalue_roll _returnvalue_pitch _returnvalue_yaw) (`KismetMathLibrary.BreakRotator` (`KismetMathLibrary.FindLookAtRotation` (`self.StartingLocation`) (`self.Destination`))))
  (set `self.Delta Apex` DeltaApex)
  (set `self.Destination` TargetLocation)
  (bind _output_get (set `self.StartingLocation` (`self.K2_GetActorLocation`)))
  (set `self.PrevLocation` _output_get)
  (`SceneComponent.K2_SetWorldRotation` (`self.StaticMesh`) (`KismetMathLibrary.MakeRotator` _returnvalue_roll (+ _returnvalue_pitch -90.0) _returnvalue_yaw) false false)
  (`TimelineComponent.SetPlayRate` (`self.MoveArrow`) (/ 1.0 FlightTime))
  (bind (_direction _newtrack_0) (`Timeline|MoveArrow` :!via `PlayFromStart`)
    (:`Update`
      (bind _returnvalue (`KismetMathLibrary.MakeVector` (.x (`KismetMathLibrary.VLerp` _startinglocation (`self.Destination`) (.x _newtrack_0))) (.y (`KismetMathLibrary.VLerp` _startinglocation (`self.Destination`) (.x _newtrack_0))) (+ (* (.z _newtrack_0) (`self.Delta Apex`)) (.z _startinglocation))))
      (`self.K2_SetActorLocation` _returnvalue)
      (bind (_returnvalue_roll_2 _returnvalue_pitch_2 _returnvalue_yaw_2) (`KismetMathLibrary.BreakRotator` (`KismetMathLibrary.FindLookAtRotation` (`self.PrevLocation`) _returnvalue)))
      (`SceneComponent.K2_SetWorldRotation` (`self.StaticMesh`) (`KismetMathLibrary.MakeRotator` _returnvalue_roll_2 (+ _returnvalue_pitch_2 -90.0) _returnvalue_yaw_2) false false)
      (set `self.PrevLocation` _returnvalue))
    (:`Finished`
      (`self.K2_DestroyActor`))))

(fn `UserConstructionScript`)