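; BP_GridSquare is a combat-level grid tile that shows hover and selection state through color.
; On BeginPlay it applies a dynamic instance of a simple grid material to its cube.
; Cursor-over events toggle a yellow highlight and SetSelected toggles a light blue tint, both via the ColorMultiplier parameter.
; Selection color takes priority over hover highlighting, and the click handler is left empty.
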(event `self.ReceiveBeginPlay`
  (bind _returnvalue (`KismetMaterialLibrary.CreateDynamicMaterialInstance` "/Game/CombatLevel/Materials/MI_GridMaterialSimple.MI_GridMaterialSimple"))
  (bind _output_get (set `self.DynamicMeshMaterial` _returnvalue))
  (`PrimitiveComponent.SetMaterial` (`self.Cube`) 0 _output_get))

(event `self.HandleGridSquareClicked`
  ;[1 1 1] Blueprint responses to mouse events
)

(event `self.HandleGridSquareBeginCursorOver`
  ;[1 1 1] Blueprint responses to mouse events
  (`self.SetHighlighted` true))

(event `self.HandleGridSquareEndCursorOver`
  ;[1 1 1] Blueprint responses to mouse events
  (`self.SetHighlighted` false))

(event `self.SetHighlighted`
  (params (isHighlighted :type Boolean))
  (bind _output_get (set `self.bIsHighlighted` isHighlighted))
  (if (not (`self.bIsSelected`))
    (`MaterialInstanceDynamic.SetVectorParameterValue` (`self.DynamicMeshMaterial`) "ColorMultiplier" (`KismetMathLibrary.SelectColor` (struct :`R` 1.0 :`G` 0.904661 :`B` 0.234551 :`A` 1.0) (struct :`R` 1.0 :`G` 1.0 :`B` 1.0 :`A` 1.0) _output_get))))

(event `self.SetSelected`
  (params (isSelected :type Boolean))
  (bind _output_get (set `self.bIsSelected` isSelected))
  (`MaterialInstanceDynamic.SetVectorParameterValue` (`self.DynamicMeshMaterial`) "ColorMultiplier" (`KismetMathLibrary.SelectColor` (struct :`R` 0.342181 :`G` 0.879903 :`B` 1.0 :`A` 1.0) (struct :`R` 1.0 :`G` 1.0 :`B` 1.0 :`A` 1.0) _output_get)))

(fn `UserConstructionScript`)