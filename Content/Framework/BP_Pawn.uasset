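; BP_Pawn is a player pawn that moves in a plane from WASD axis input.
; MoveRight and MoveUp add movement input along the actor's right and forward vectors.
; ScaleAxisValue multiplies each input by the zoom target index plus one, over the count of spring arm zoom lengths, so movement strength follows the zoom step.
; The file reads the zoom state but does not change it.
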(event `self.ReceiveTick`
  (params (DeltaSeconds :type "Float (single-precision)")))

(event `InputAxis|MoveRight`
  (params (AxisValue :type "Float (single-precision)"))
  ;[1 0.625 0.625] Handle WASD movement in plane
  (bind _scaledvalue (`self.ScaleAxisValue` AxisValue))
  (`self.AddMovementInput` (`self.GetActorRightVector`) _scaledvalue))

(event `InputAxis|MoveUp`
  (params (AxisValue :type "Float (single-precision)"))
  ;[1 0.625 0.625] Handle WASD movement in plane
  (bind _scaledvalue (`self.ScaleAxisValue` AxisValue))
  (`self.AddMovementInput` (`self.GetActorForwardVector`) _scaledvalue))

(fn `ScaleAxisValue`
  (params (OriginalValue :type "Float (double-precision)"))
  (returns (ScaledValue :type "Float (double-precision)"))
  (return (* OriginalValue (/ (`KismetMathLibrary.Conv_IntToDouble` (+ (`self.ZoomTargetIndex`) 1)) (`KismetMathLibrary.Conv_IntToDouble` (`KismetArrayLibrary.Array_Length` (`self.SpringArmZoomLengths`)))))))

(fn `UserConstructionScript`)