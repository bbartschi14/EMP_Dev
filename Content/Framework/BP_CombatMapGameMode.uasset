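; Combat map game mode that runs end-of-turn simulation of queued actions and squad-versus-squad combat.
; EndTurn enters the simulating state and executes queued actions sequentially, advancing on each action's finished event until the queue empties.
; InitiateCombat creates a combat simulator, and CombatRound recursively times attacks, damage and movement with delays, then resets units, resolves morale and signals completion.
; A disconnected squad-movement check remains in the graph but never runs.
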(event `self.InitiateCombat`
  (params (squadOne :type "EMPSquadData Object Reference") (squadTwo :type "EMPSquadData Object Reference"))
  ;[0.3364 0.4742 1] Combat Simulation
  (bind _returnvalue (`self.SetupCombat` squadOne squadTwo))
  (set `self.CombatSimulator` _returnvalue)
  (`self.CombatRound`))

(event `CombatRound`
  (bind _combatsimulator (`self.CombatSimulator`))
  (bind _returnvalue (/ 1.2 2.0))
  ;[0.3364 0.4742 1] Combat Simulation
  (`EMPCombatSimulator.SimulateSingleRoundOfAttacks` _combatsimulator)
  (bind _returnvalue_2 (`EMPCombatSimulator.AnimateAttacks` _combatsimulator 1.2))
  (if _returnvalue_2
    (`KismetSystemLibrary.Delay` _returnvalue) ; Only delay if any attacks are waiting
    (`EMPCombatSimulator.ResolveDamage` _combatsimulator)
    (`KismetSystemLibrary.Delay` _returnvalue))
  (`EMPCombatSimulator.UpdateCombatMovement` _combatsimulator 0.5)
  (`KismetSystemLibrary.Delay` 0.5)
  (bind _result (`/Engine/EditorBlueprintResources/StandardMacros.DecrementInt` (`EMPCombatSimulator.CombatRoundsRemaining` _combatsimulator))
    (:`  `
      (if (> _result 0)
        (`self.CombatRound`)
        (else
          (`EMPCombatSimulator.ResetCombatUnitsAfterCombat` _combatsimulator 0.5)
          (`KismetSystemLibrary.Delay` 0.5)
          ;[1 0.7007 0.1978 1 20] Do Morale rolls
          (`EMPCombatSimulator.PerformMoraleRolls` _combatsimulator 2.0)
          (`KismetSystemLibrary.Delay` 2.0)
          (bind _returnvalue_3 (`EMPCombatSimulator.ResolveMoraleRolls` _combatsimulator 1.0))
          (if _returnvalue_3
            (`KismetSystemLibrary.Delay` 1.0))
          ;[1 1 1] Return to action queue
          (set `self.CombatSimulator` null)
          (`self.OnCombatSimuationFinished`))))))

(event `self.EndTurn`
  (bind _asempplayer_controller (cast `EMPPlayerController` (`GameplayStatics.GetPlayerController` 0)))
  (`EMPPlayerController.HandleCancelActionPressed` _asempplayer_controller)
  (if (`|EnumInequality` (`self.CurrentState`) "GS_SIMULATING")
    (`self.SetCombatMapState` "GS_SIMULATING")
    (`self.ResolveCurrentAction`)))

(event `ResolveCurrentAction`
  (bind _output (`|GetArrayItem` (`self.QueuedActions`)))
  (if (> (`KismetArrayLibrary.Array_Length` (`self.QueuedActions`)) 0)
    (`self.OnActionStarted` _output)
    (add `EMPCombatActionSkill.OnCombatActionFinishedExecuting` _output (delegate `OnFinishedExecuting`))
    (`EMPCombatActionSkill.ExecuteAction` _output)
    (else
      (`self.FinishSimulating`))))

(event `OnFinishedExecuting`
  (params (Action :type "EMPCombatActionSkill Object Reference"))
  (remove `EMPCombatActionSkill.OnCombatActionFinishedExecuting` Action (delegate `OnFinishedExecuting`))
  (`self.HandleActionFinished`))

(event `HandleActionFinished`
  (`self.OnActionCompleted` null)
  (`KismetArrayLibrary.Array_Remove` (`self.QueuedActions`))
  (`self.OnActionQueuePopped`)
  (`self.ResolveCurrentAction`))

(fn `UserConstructionScript`)