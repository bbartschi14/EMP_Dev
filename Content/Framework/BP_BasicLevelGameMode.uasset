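; Basic level game mode that spawns friendly and enemy squads for combat from the EMP squad manager's saved squad data.
; LoadFriendlySquads loads squad entries 0 through 2 for the friendly player, placing them in area column X=0 with the row matching the index.
; LoadEnemySquads reuses the same data array but loads only entry 2, at column X=2.
; Both skip missing indices; BeginPlay, Tick and construction are empty.
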(event `self.ReceiveBeginPlay`)

(event `self.LoadFriendlySquads`
  (params (friendlyPlayer :type "EMPCombatPlayer Object Reference"))
  (bind _returnvalue (`EMPSquadManager.GetSquadData` (subsystem `EMPSquadManager`)))
  (for _index (range 3)
    (if (`KismetArrayLibrary.Array_IsValidIndex` _returnvalue _index)
      (`self.LoadSquad` friendlyPlayer (`|GetArrayItem` _returnvalue _index) (make `IntPoint` 0 _index)))))

(event `self.LoadEnemySquads`
  (params (enemyPlayer :type "EMPCombatPlayer Object Reference"))
  (bind _returnvalue (`EMPSquadManager.GetSquadData` (subsystem `EMPSquadManager`)))
  (for _index (range 2 3)
    (if (`KismetArrayLibrary.Array_IsValidIndex` _returnvalue _index)
      (`self.LoadSquad` enemyPlayer (`|GetArrayItem` _returnvalue _index) (make `IntPoint` 2 _index)))))

(fn `UserConstructionScript`)