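; Combat-map actor that represents one squad on the grid and hosts its quick-menu widget.
; It snaps to the world location of the squad data's combat area at start and whenever that data reports a move.
; Game mode select and deselect events drive its selected state, which it forwards to the quick menu.
; Selection requires a match with its own squad data, while any deselect event clears it.
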(event `self.ReceiveBeginPlay`
  (add `EMPSquadData.OnSquadMovedToAreaLocation` (`self.OwningSquadData`) (delegate `OnSquadMovedToAreaLocation_Event_0`))
  (`self.UpdatePosition`)
  (bind _asbp_combat_map_game_mode (cast `/Game/Framework/BP_CombatMapGameMode` (`GameplayStatics.GetGameMode`)))
  (add `EMPCombatMapGameMode.OnSquadSelected` _asbp_combat_map_game_mode (delegate `OnSquadSelected_Event_0`))
  (add `EMPCombatMapGameMode.OnSquadDeselected` _asbp_combat_map_game_mode (delegate `OnSquadDeselected_Event_0`))
  (bind _aswbp_squad_quick_menu (cast `/Game/UI/CombatMap/QuickMenu/WBP_SquadQuickMenu` (`WidgetComponent.GetUserWidgetObject` (`self.Widget`))))
  (bind _output_get (set `self.As WBP Squad Quick Menu` _aswbp_squad_quick_menu))
  (`/Game/UI/CombatMap/QuickMenu/WBP_SquadQuickMenu.SetSquad` _output_get (`self.OwningSquadData`)))

(event `OnSquadMovedToAreaLocation_Event_0`
  (`self.UpdatePosition`))

(event `OnSquadSelected_Event_0`
  (params (squadData :type "EMPSquadData Object Reference"))
  (if (== squadData (`self.OwningSquadData`))
    (`self.SetSelected` true)))

(event `OnSquadDeselected_Event_0`
  (`self.SetSelected` false))

(event `UpdatePosition`
  (`self.K2_SetActorLocation` (`EMPGrid.GetWorldLocationFromGridArea` (`self.OwningGrid`) (`EMPSquadData.GetCombatAreaLocation` (`self.OwningSquadData`)))))

(event `SetSelected`
  (params (IsSelected :type Boolean))
  (if (not (== IsSelected (`self.IsSelected`)))
    (bind _output_get (set `self.IsSelected` IsSelected))
    (`/Game/UI/CombatMap/QuickMenu/WBP_SquadQuickMenu.SetSelected` (`self.As WBP Squad Quick Menu`) _output_get)))

(fn `UserConstructionScript`)