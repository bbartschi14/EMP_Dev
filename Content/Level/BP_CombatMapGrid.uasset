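; BP_CombatMapGrid is the combat map's grid actor, turning square clicks and hovers into squad selection, movement and unit rearrangement.
; Input branches on the game mode's map state, highlighting 5x5 areas and limiting squad moves by reachability and height difference.
; It binds game mode events on BeginPlay to animate, turn, ready and remove unit actors, and spawns spline arrows for queued moves.
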(event `HandleActionQueued`
  (params (actionData :type "EMPCombatActionData Object Reference"))
  (bind _asempmovement_action_data (cast `EMPMovementActionData` actionData))
  (bind _location (`self.GetWorldLocationCenterOfArea` (`EMPSquadData.CombatAreaLocation` (`EMPMovementActionData.SquadToMove` _asempmovement_action_data))))
  (bind _location_2 (`self.GetWorldLocationCenterOfArea` (`EMPMovementActionData.Destination` _asempmovement_action_data)))
  (bind _returnvalue (`|SpawnActorFromClass` "/Game/Level/BP_ArrowSplineMesh.BP_ArrowSplineMesh_C" (`KismetMathLibrary.MakeTransform` (0.0 0.0 50.0)) "Undefined" "OverrideRootScale" null null))
  (`EMPArrowSplineMesh.InitializeArrow` _returnvalue _location _location_2 _asempmovement_action_data))

(event `self.ReceiveBeginPlay`
  (bind _asbp_combat_map_game_mode (`self.GetCombatMapGameMode`))
  (add `EMPCombatMapGameMode.OnSquadSelected` _asbp_combat_map_game_mode (`|CreateDelegate` :!event `OnSquadSelected`))
  (add `EMPCombatMapGameMode.OnSquadDeselected` _asbp_combat_map_game_mode (`|CreateDelegate` :!event `OnSquadDeselected`))
  (add `EMPCombatMapGameMode.OnCombatUnitMoved` _asbp_combat_map_game_mode (`|CreateDelegate` :!event `OnCombatUnitMoved`))
  (add `EMPCombatMapGameMode.OnCombatUnitMovementFailed` _asbp_combat_map_game_mode (`|CreateDelegate` :!event `OnCombatUnitMovementFailed`))
  (add `EMPCombatMapGameMode.OnCombatUnitDied` _asbp_combat_map_game_mode (`|CreateDelegate` :!event `OnCombatUnitDied`))
  (add `EMPCombatMapGameMode.OnCombatUnitAttackAnimate` _asbp_combat_map_game_mode (`|CreateDelegate` :!event `OnCombatUnitAttackAnimate`))
  (add `EMPCombatMapGameMode.OnCombatUnitSelected` _asbp_combat_map_game_mode (`|CreateDelegate` :!event `OnCombatUnitSelected`))
  (add `EMPCombatMapGameMode.OnCombatUnitDeselected` _asbp_combat_map_game_mode (`|CreateDelegate` :!event `OnCombatUnitDeselected`))
  (add `EMPCombatMapGameMode.OnCombatInitiated` _asbp_combat_map_game_mode (`|CreateDelegate` :!event `OnCombatInitiated`))
  (add `EMPCombatMapGameMode.OnCombatEnded` _asbp_combat_map_game_mode (`|CreateDelegate` :!event `OnCombatEnded`))
  (add `EMPCombatMapGameMode.OnActionQueued` _asbp_combat_map_game_mode (`|CreateDelegate` :!event `HandleActionQueued`))
  (add `EMPCombatMapGameMode.OnCombatUnitRetreat` _asbp_combat_map_game_mode (`|CreateDelegate` :!event `OnCombatUnitRetreat`)))

(event `self.OnGridSquareClicked`
  (params (inGridSquare :type "EMPGridSquare Object Reference"))
  ;[1 1 1] Click
  (bind _asbp_combat_map_game_mode (`self.GetCombatMapGameMode`))
  (`self.SwitchOnCombatMapState` (`EMPCombatMapGameMode.GetCombatMapState` _asbp_combat_map_game_mode)
    (:`SelectingSquad`
      (`self.TrySelectSquad` _asbp_combat_map_game_mode inGridSquare))
    (:`MovingSquad`
      (`self.TryMoveSelectedSquad` _asbp_combat_map_game_mode inGridSquare))
    (:`RearrangingSquad`
      (`self.TrySelectCombatUnit` _asbp_combat_map_game_mode inGridSquare))))

(event `OnCombatInitiated`
  (params (squadOne :type "EMPSquadData Object Reference") (squadTwo :type "EMPSquadData Object Reference"))
  (bind _combatarealocation (`EMPSquadData.CombatAreaLocation` squadTwo))
  (bind _combatarealocation_2 (`EMPSquadData.CombatAreaLocation` squadOne))
  (bind _returnvalue (`EMPCombatStatics.IntPointToDirection` (- _combatarealocation _combatarealocation_2)))
  (`self.TurnCombatUnitsInSquadToDirection` squadOne _returnvalue)
  (bind _returnvalue_2 (`EMPCombatStatics.IntPointToDirection` (- _combatarealocation_2 _combatarealocation)))
  (`self.TurnCombatUnitsInSquadToDirection` squadTwo _returnvalue_2)
  (`self.SetCombatUnitsInSquadReady` squadTwo true)
  (`self.SetCombatUnitsInSquadReady` squadOne true))

(event `OnSquadSelected`
  (params (squadData :type "EMPSquadData Object Reference"))
  (bind _output_get (set `self.SelectedSquad` squadData))
  (`self.HandleSetGridAreaSelected` (`EMPSquadData.CombatAreaLocation` _output_get) true))

(event `self.OnGridSquareRightClicked`
  (params (inGridSquare :type "EMPGridSquare Object Reference"))
  ;[1 1 1] Click
  (bind _asbp_combat_map_game_mode (`self.GetCombatMapGameMode`))
  (`self.SwitchOnCombatMapState` (`EMPCombatMapGameMode.GetCombatMapState` _asbp_combat_map_game_mode)
    (:`RearrangingSquad`
      (if (`KismetSystemLibrary.IsValid` (`self.SelectedCombatUnit`))
        (`self.TryRearrangeCombatUnit` _asbp_combat_map_game_mode inGridSquare)))))

(event `OnCombatUnitMoved`
  (params (combatUnit :type "EMPCombatUnitData Object Reference") (animationTime :type "Float (double-precision)"))
  (bind _returnvalue (`self.GetCombatUnitFromData` combatUnit))
  (if (`KismetSystemLibrary.IsValid` _returnvalue)
    (`EMPCombatUnit.MoveToGridSquare_Timed` _returnvalue (`EMPCombatUnitData.CombatLocation` combatUnit) animationTime)))

(event `OnSquadDeselected`
  (`self.HandleSetGridAreaSelected` (`EMPSquadData.CombatAreaLocation` (`self.SelectedSquad`))))

(event `self.OnGridSquareHovered`
  (params (inGridSquare :type "EMPGridSquare Object Reference"))
  (bind _asbp_combat_map_game_mode (`self.GetCombatMapGameMode`))
  (`self.SwitchOnCombatMapState` (`EMPCombatMapGameMode.GetCombatMapState` _asbp_combat_map_game_mode)
    (:`SelectingSquad`
      (`self.IsFriendlySquadAtGridSquare` inGridSquare
        (:`Found`
          (`self.HandleSetGridAreaHighlighted` (`self.GetAreaCoordinateOfGridCoordinate` (`EMPGridSquare.GridCoordinate` inGridSquare)) true))))
    (:`MovingSquad`
      (bind _newlocation (`self.CanSelectedSquadMoveToGridSquare` inGridSquare)
        (:`true`
          (`self.HandleSetGridAreaHighlighted` _newlocation true))))))

(event `OnCombatEnded`
  (params (squadOne :type "EMPSquadData Object Reference") (squadTwo :type "EMPSquadData Object Reference"))
  (`self.TurnCombatUnitsInSquadToDefaultDirection` squadOne)
  (`self.TurnCombatUnitsInSquadToDefaultDirection` squadTwo)
  (`self.SetCombatUnitsInSquadReady` squadTwo)
  (`self.SetCombatUnitsInSquadReady` squadOne))

(event `TrySelectCombatUnit`
  (params (CombatMap :type "/Game/Framework/BP_CombatMapGameMode Object Reference") (GridSquare :type "EMPGridSquare Object Reference"))
  ;[1 1 1] Click
  (bind _returnvalue (`EMPSquadData.GetCombatUnitAtCombatLocation` (`self.SelectedSquad`) (`EMPGridSquare.GridCoordinate` GridSquare)))
  (if (`KismetSystemLibrary.IsValid` _returnvalue)
    (`EMPCombatMapGameMode.SelectCombatUnit` CombatMap _returnvalue)))

(event `TrySelectSquad`
  (params (CombatMap :type "/Game/Framework/BP_CombatMapGameMode Object Reference") (GridSquare :type "EMPGridSquare Object Reference"))
  ;[1 1 1] Click
  (bind _squad (`self.IsFriendlySquadAtGridSquare` GridSquare)
    (:`Found`
      (`EMPCombatMapGameMode.SelectSquad` CombatMap _squad))))

(event `OnCombatUnitMovementFailed`
  (params (combatUnit :type "EMPCombatUnitData Object Reference") (animationTime :type "Float (double-precision)"))
  (bind _returnvalue (`self.GetCombatUnitFromData` combatUnit))
  (if (`KismetSystemLibrary.IsValid` _returnvalue)
    (`EMPCombatUnit.HandleMovementFailed_Timed` _returnvalue animationTime)))

(event `OnCombatUnitDied`
  (params (combatUnit :type "EMPCombatUnitData Object Reference"))
  (bind _returnvalue (`self.GetCombatUnitFromData` combatUnit))
  (if (`KismetSystemLibrary.IsValid` _returnvalue)
    (`self.K2_DestroyActor` _returnvalue)
    (`KismetArrayLibrary.Array_RemoveItem` (`self.CombatUnits`) _returnvalue)))

(event `TryRearrangeCombatUnit`
  (params (CombatMap :type "/Game/Framework/BP_CombatMapGameMode Object Reference") (GridSquare :type "EMPGridSquare Object Reference"))
  ;[1 1 1] Click
  (`EMPCombatMapGameMode.RearrangeCombatUnitToLocation` CombatMap (`self.SelectedCombatUnit`) (`EMPGridSquare.GridCoordinate` GridSquare) 0.5))

(event `TryMoveSelectedSquad`
  (params (CombatMap :type "/Game/Framework/BP_CombatMapGameMode Object Reference") (GridSquare :type "EMPGridSquare Object Reference"))
  ;[1 1 1] Click
  (bind _newlocation (`self.CanSelectedSquadMoveToGridSquare` GridSquare)
    (:`true`
      (`EMPCombatMapGameMode.QueueAction_MoveSelectedSquad` CombatMap _newlocation))))

(event `self.OnGridSquareUnhovered`
  (params (inGridSquare :type "EMPGridSquare Object Reference"))
  (`self.HandleSetGridAreaHighlighted` (`self.GetAreaCoordinateOfGridCoordinate` (`EMPGridSquare.GridCoordinate` inGridSquare))))

(event `OnCombatUnitAttackAnimate`
  (params (attackingCombatUnit :type "EMPCombatUnitData Object Reference") (defendingCombatUnit :type "EMPCombatUnitData Object Reference") (animationTime :type "Float (double-precision)"))
  (bind _returnvalue (`self.GetCombatUnitFromData` defendingCombatUnit))
  (bind _returnvalue_2 (`self.GetCombatUnitFromData` attackingCombatUnit))
  (if (and (`KismetSystemLibrary.IsValid` _returnvalue) (`KismetSystemLibrary.IsValid` _returnvalue_2))
    (`EMPCombatUnit.SetAttackTargetLocation` _returnvalue_2 (`self.K2_GetActorLocation` _returnvalue))
    (`EMPCombatUnit.TriggerAttack` _returnvalue_2)))

(event `OnCombatUnitSelected`
  (params (combatUnit :type "EMPCombatUnitData Object Reference"))
  (bind _output_get (set `self.SelectedCombatUnit` combatUnit))
  (bind _returnvalue (`self.GetCombatUnitFromData` _output_get))
  (if (`KismetSystemLibrary.IsValid` _returnvalue)
    (bind _asbp_combat_unit (cast `/Game/Combat/BP_CombatUnit` _returnvalue))
    (`EMPCombatUnit.SetReadyStance` _asbp_combat_unit true)))

(event `OnCombatUnitDeselected`
  (bind _returnvalue (`self.GetCombatUnitFromData` (`self.SelectedCombatUnit`)))
  (if (`KismetSystemLibrary.IsValid` _returnvalue)
    (bind _asbp_combat_unit (cast `/Game/Combat/BP_CombatUnit` _returnvalue))
    (`EMPCombatUnit.SetReadyStance` _asbp_combat_unit false)
    (set `self.SelectedCombatUnit` null)))

(event `OnCombatUnitRetreat`
  (params (combatUnit :type "EMPCombatUnitData Object Reference") (animationTime :type "Float (double-precision)"))
  (bind _returnvalue (`self.GetCombatUnitFromData` combatUnit))
  (if (`KismetSystemLibrary.IsValid` _returnvalue)
    (bind _asbp_combat_unit (cast `/Game/Combat/BP_CombatUnit` _returnvalue))
    (`/Game/Combat/BP_CombatUnit.RetreatCombatUnit` _asbp_combat_unit animationTime)
    (`KismetArrayLibrary.Array_RemoveItem` (`self.CombatUnits`) _returnvalue)))

(fn `UserConstructionScript`)