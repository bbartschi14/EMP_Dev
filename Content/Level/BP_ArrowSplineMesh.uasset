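; BP_ArrowSplineMesh is an arrow actor on the combat map that spans two locations and is tied to an owning action.
; InitializeArrow sets the spline mesh's endpoints and gives both tangents the start-to-end vector, forming a straight segment.
; It then binds to the action-started event on BP_CombatMapGameMode and destroys itself when the started action matches its owning action.
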(event `self.InitializeArrow`
  (params (startLocation :type "Vector Structure") (endLocatiion :type "Vector Structure") (owningAction :type "EMPCombatActionData Object Reference"))
  (bind _returnvalue (- endLocatiion startLocation))
  (bind _splinemesh (`self.SplineMesh`))
  (set `self.OwningAction` owningAction)
  (`SplineMeshComponent.SetStartPosition` _splinemesh startLocation false)
  (`SplineMeshComponent.SetEndPosition` _splinemesh endLocatiion true)
  (`SplineMeshComponent.SetStartTangent` _splinemesh _returnvalue false)
  (`SplineMeshComponent.SetEndTangent` _splinemesh _returnvalue true)
  (bind _asbp_combat_map_game_mode (cast `/Game/Framework/BP_CombatMapGameMode` (`GameplayStatics.GetGameMode`)))
  (add `EMPCombatMapGameMode.OnActionStarted` _asbp_combat_map_game_mode (delegate `OnActionStarted`)))

(event `OnActionStarted`
  (params (actionData :type "EMPCombatActionData Object Reference"))
  (if (== (`self.OwningAction`) actionData)
    (`self.CleanupAndDestroy`)))

(event `CleanupAndDestroy`
  (`self.K2_DestroyActor`))

(fn `UserConstructionScript`)