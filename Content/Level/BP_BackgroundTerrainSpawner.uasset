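; BP_BackgroundTerrainSpawner scatters hundreds of terrain mesh instances at runtime to form background scenery.
; On BeginPlay it creates a dynamic instance of M_BackgroundTerrain, tints it with PlaneColor and assigns it to an InstancedStaticMesh component.
; A loop then adds instances with random position, slight roll and yaw, and varied scale, each composed with the component's world transform.
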(event `self.ReceiveBeginPlay`
  (bind _returnvalue (`KismetMathLibrary.RandomFloatInRange` 0.0 4.0))
  (bind _instancedstaticmesh (`self.InstancedStaticMesh`))
  (bind _returnvalue_2 (* -1 8000.0))
  (bind _returnvalue_3 (`KismetMaterialLibrary.CreateDynamicMaterialInstance` "/Game/Materials/M_BackgroundTerrain.M_BackgroundTerrain"))
  (`MaterialInstanceDynamic.SetVectorParameterValue` _returnvalue_3 "Color" (`self.PlaneColor`))
  (`PrimitiveComponent.SetMaterial` (`self.InstancedStaticMesh`) 0 _returnvalue_3)
  (for _ (range 801)
    (`InstancedStaticMeshComponent.AddInstance` _instancedstaticmesh (`KismetMathLibrary.ComposeTransforms` (`KismetMathLibrary.MakeTransform` (`KismetMathLibrary.MakeVector` (`KismetMathLibrary.RandomFloatInRange` _returnvalue_2 8000.0) (`KismetMathLibrary.RandomFloatInRange` _returnvalue_2 8000.0) (`KismetMathLibrary.RandomFloatInRange` -4000.0 500.0)) (`KismetMathLibrary.MakeRotator` (`KismetMathLibrary.RandomFloatInRange` -5.0 5.0) 0.0 (`KismetMathLibrary.RandomFloatInRange` -5.0 5.0)) (+ (`KismetMathLibrary.MakeVector` 4.0 4.0 4.0) (`KismetMathLibrary.MakeVector` _returnvalue _returnvalue _returnvalue))) (`SceneComponent.K2_GetComponentToWorld` _instancedstaticmesh)))))

(event `self.ReceiveTick`
  (params (DeltaSeconds :type "Float (single-precision)")))

(fn `UserConstructionScript`)