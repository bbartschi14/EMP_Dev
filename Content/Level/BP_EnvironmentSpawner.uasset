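; BP_EnvironmentSpawner scatters instanced grass across the 2D bounds of the level's EMPGrid at BeginPlay.
; It creates a FastNoise wrapper, finds the grid and waits a zero-length Delay before spawning.
; SpawnGrass makes random placement attempts in proportion to grid area and density, keeping points whose remapped noise exceeds a threshold.
; Each instance gets random yaw and a noise-driven scale with random variation.
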(event `self.ReceiveBeginPlay`
  (bind _returnvalue (`|GenericCreateObject` "/Script/FastNoiseGenerator.FastNoiseWrapper" self))
  (bind _output_get (set `self.Noise` _returnvalue))
  (`FastNoiseWrapper.SetupFastNoise` _output_get "Simplex" 1337 0.002 "Quintic" "FBM" 2 2.0 0.5 0.1 "Euclidean" "CellValue")
  (bind _returnvalue_2 (`GameplayStatics.GetActorOfClass` "/Script/EmpireDEV.EMPGrid"))
  (`KismetSystemLibrary.Delay` 0.0)
  (`self.Spawn` _returnvalue_2))

(event `Spawn`
  (params (Grid :type "EMPGrid Object Reference"))
  (`self.SpawnGrass` 0.6 Grid))

(event `SpawnGrass`
  (params (GrassDensity :type "Float (double-precision)") (Grid :type "EMPGrid Object Reference"))
  (bind (_min _max) (`EMPGrid.Get2DBounds` Grid))
  (bind _returnvalue (`KismetMathLibrary.MapRangeClamped` (`FastNoiseWrapper.GetNoise2D` (`self.Noise`) (`self.RandomX`) (`self.RandomY`)) -1.0 1.0 0.0 1.0))
  (for _ (range (+ (`KismetMathLibrary.FTrunc` (* (* (- (`KismetMathLibrary.BreakVector2D` _max) (`KismetMathLibrary.BreakVector2D` _min)) (- (`.Y` (`KismetMathLibrary.BreakVector2D` _max)) (`.Y` (`KismetMathLibrary.BreakVector2D` _min)))) (* GrassDensity 0.01))) 1))
    (set `self.RandomX` (`KismetMathLibrary.RandomFloatInRange` (`KismetMathLibrary.BreakVector2D` _min) (- (`KismetMathLibrary.BreakVector2D` _max) 20.0)))
    (set `self.RandomY` (`KismetMathLibrary.RandomFloatInRange` (`.Y` (`KismetMathLibrary.BreakVector2D` _min)) (- (`.Y` (`KismetMathLibrary.BreakVector2D` _max)) 20.0)))
    (if (> _returnvalue 0.2)
      (`InstancedStaticMeshComponent.AddInstanceWorldSpace` (`self.GrassInstances`) (`KismetMathLibrary.MakeTransform` (`KismetMathLibrary.MakeVector` (`self.RandomX`) (`self.RandomY`)) (`KismetMathLibrary.MakeRotator` 0.0 0.0 (`KismetMathLibrary.RandomFloatInRange` 0.0 360.0)) (`KismetMathLibrary.Conv_DoubleToVector` (* (* 1 _returnvalue) (`KismetMathLibrary.RandomFloatInRange` 0.8 1.3))))))))

(fn `UserConstructionScript`)