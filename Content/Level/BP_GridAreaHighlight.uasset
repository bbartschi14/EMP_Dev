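; Grid area highlight Blueprint that tints a decal to show an area's hover and selection state.
; BeginPlay creates a dynamic material instance from the decal, then RefreshVisuals uses a branching helper on IsSelected and IsHovered to set visibility, color and brightness parameters.
; IsForceVisible is applied last, so it overrides every state with a visible off-white look.
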(event `self.ReceiveBeginPlay`
  (bind _returnvalue (`DecalComponent.CreateDynamicMaterialInstance` (`self.Decal`)))
  (set `self.DynamicGridMaterial` _returnvalue)
  (`self.RefreshVisuals`))

(event `self.RefreshVisuals`
  (`|ExecutionSequence`
    (:`then_0`
      (`self.SwitchOnVisualStyle`
        (:`Selected AND Hovered`
          (`self.SetGridMaterialParameters` 1.0 (struct :`G` 0.577581 :`B` 1.0 :`A` 1.0) 3.0))
        (:`Selected but NOT Hovered`
          (`self.SetGridMaterialParameters` 1.0 (struct :`G` 0.577581 :`B` 1.0 :`A` 1.0) 2.0))
        (:`Hovered but NOT Selected`
          (`self.SetGridMaterialParameters` 1.0 (struct :`R` 1.0 :`G` 1.0 :`B` 1.0 :`A` 1.0) 2.0))
        (:`NOT Hovered and NOT Selected`
          (`self.SetGridMaterialParameters` 0.0 (struct :`R` 0.165132 :`G` 0.165132 :`B` 0.165132 :`A` 1.0) 0.5))))
    (:`then_1`
      (if (`self.bIsForceVisible`)
        (`self.SetGridMaterialParameters` 1.0 (struct :`R` 0.921875 :`G` 0.921875 :`B` 0.921875 :`A` 1.0) 1.0)))))

(fn `UserConstructionScript`)