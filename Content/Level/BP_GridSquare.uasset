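; BP_GridSquare is a single square of a level grid that gives visual feedback for cursor hover and selection.
; BeginPlay creates dynamic material instances for the cube and decal, but only the decal's is animated by state changes.
; Hover raises decal brightness and forces visibility, with updates skipped while selected.
; Selection recolors the decal and reapplies the current highlight state; the click handler is empty.
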(event `self.ReceiveBeginPlay`
  (`|ExecutionSequence`
    (:`then_0`
      (bind _returnvalue (`KismetMaterialLibrary.CreateDynamicMaterialInstance` "/Game/Level/Materials/MI_GridMaterialSimple.MI_GridMaterialSimple"))
      (bind _output_get (set `self.DynamicMeshMaterial` _returnvalue))
      (`PrimitiveComponent.SetMaterial` (`self.Cube`) 0 _output_get))
    (:`then_1`
      (bind _returnvalue_2 (`DecalComponent.CreateDynamicMaterialInstance` (`self.Decal`)))
      (set `self.DynamicGridMaterial` _returnvalue_2))))

(event `self.HandleGridSquareClicked`
  ;[1 1 1] Blueprint responses to mouse events
)

(event `self.HandleGridSquareBeginCursorOver`
  ;[1 1 1] Blueprint responses to mouse events
  (`self.SetHighlighted` true))

(event `self.HandleGridSquareEndCursorOver`
  ;[1 1 1] Blueprint responses to mouse events
  (`self.SetHighlighted` false))

(event `self.SetHighlighted`
  (params (isHighlighted :type Boolean))
  (bind _output_get (set `self.bIsHighlighted` isHighlighted))
  (if (not (`self.bIsSelected`))
    (`MaterialInstanceDynamic.SetScalarParameterValue` (`self.DynamicGridMaterial`) "Brightness" (`KismetMathLibrary.SelectFloat` 4.0 0.75 _output_get) :!label _label)
    (`MaterialInstanceDynamic.SetScalarParameterValue` (`self.DynamicGridMaterial`) "ForceVisible" (`KismetMathLibrary.SelectFloat` 1.0 0.0 _output_get))))

(event `self.SetSelected`
  (params (isSelected :type Boolean))
  (bind _output_get (set `self.bIsSelected` isSelected))
  (`MaterialInstanceDynamic.SetVectorParameterValue` (`self.DynamicGridMaterial`) "Color" (`KismetMathLibrary.SelectColor` (struct :`G` 0.57265 :`B` 1.0 :`A` 1.0) (struct :`R` 1.0 :`G` 1.0 :`B` 1.0 :`A` 1.0) _output_get))
  (goto _label))

(fn `UserConstructionScript`)