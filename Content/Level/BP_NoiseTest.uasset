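; BP_NoiseTest is a test actor that visualizes 2D Perlin noise as a grid of instanced meshes with varying height.
; Its construction script creates a FastNoiseWrapper using the Freq variable, clears the instanced static mesh, then rebuilds the grid at Spacing intervals.
; Noise sampled at each grid position is remapped to drive that instance's Z scale, and each raw sample is printed.
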(fn `UserConstructionScript`
  (bind _returnvalue (`KismetSystemLibrary.MakeLiteralDouble` (`self.Spacing`)))
  (bind _returnvalue_2 (`|GenericCreateObject` "/Script/FastNoiseGenerator.FastNoiseWrapper" self))
  (bind _output_get (set `self.Noise` _returnvalue_2))
  (`FastNoiseWrapper.SetupFastNoise` _output_get "Perlin" 1337 (`self.Freq`) "Quintic" "FBM" 2 2.0 0.5 0.1 "Euclidean" "CellValue")
  (`InstancedStaticMeshComponent.ClearInstances` (`self.InstancedStaticMesh`))
  (for _index (range (+ 20 1))
    (for _index_2 (range (+ 20 1))
      (bind _returnvalue_3 (* _index _returnvalue))
      (bind _returnvalue_4 (* _index_2 _returnvalue))
      (bind _returnvalue_5 (`FastNoiseWrapper.GetNoise2D` (`self.Noise`) _returnvalue_3 _returnvalue_4))
      (`KismetSystemLibrary.PrintString` (`KismetStringLibrary.Conv_DoubleToString` _returnvalue_5))
      (`InstancedStaticMeshComponent.AddInstance` (`self.InstancedStaticMesh`) (`KismetMathLibrary.MakeTransform` (`KismetMathLibrary.MakeVector` _returnvalue_3 _returnvalue_4 0.0) (struct) (`KismetMathLibrary.MakeVector` 1.0 1.0 (* (`KismetMathLibrary.MapRangeClamped` _returnvalue_5 -1.0 1.0 0.0 1.0) 100.0)))))))