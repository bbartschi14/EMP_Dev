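; Base camp grid that displays the selected squad's combat units and lets the player select and reposition them.
; It binds to game mode selection and hover events to spawn the squad with a staggered delay, clear it, and mark grid squares.
; Left-click selects through the game mode; right-click sends moves to the squad manager.
; Squad manager events then drive timed moves, spawns and removals for the displayed squad.
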(event `self.ReceiveBeginPlay`
  (bind _returnvalue (subsystem `EMPSquadManager`))
  (`parent.ReceiveBeginPlay`)
  (bind _asbp_base_camp_game_mode (cast `/Game/Framework/BP_BaseCampGameMode` (`GameplayStatics.GetGameMode`)))
  (add `EMPBaseCampGameMode.OnSquadSelected` _asbp_base_camp_game_mode (`|CreateDelegate` :!event `HandleOnSquadSelected`))
  (add `EMPBaseCampGameMode.OnSquadDeselected` _asbp_base_camp_game_mode (`|CreateDelegate` :!event `HandleOnSquadDeselected`))
  (add `EMPBaseCampGameMode.OnCombatUnitSelected` _asbp_base_camp_game_mode (`|CreateDelegate` :!event `HandleOnCombatUnitSelected`))
  (add `EMPBaseCampGameMode.OnCombatUnitDeselected` _asbp_base_camp_game_mode (`|CreateDelegate` :!event `HandleOnCombatUnitDeselected`))
  (add `EMPBaseCampGameMode.OnCombatUnitHovered` _asbp_base_camp_game_mode (`|CreateDelegate` :!event `HandleOnCombatUnitHovered`))
  (add `EMPBaseCampGameMode.OnCombatUnitUnhovered` _asbp_base_camp_game_mode (`|CreateDelegate` :!event `HandleOnCombatUnitUnhovered`))
  (add `EMPSquadManager.OnCombatUnitRemovedFromSquad` _returnvalue (`|CreateDelegate` :!event `HandleOnCombatUnitRemovedFromSquad`))
  (add `EMPSquadManager.OnCombatUnitAssignedToSquad` _returnvalue (`|CreateDelegate` :!event `HandleOnCombatUnitAssignedToSquad`))
  (add `EMPSquadManager.OnCombatUnitMovedToNewDesiredLocation` _returnvalue (`|CreateDelegate` :!event `HandleOnCombatUnitMovedToNewDesiredLocation`)))

(event `self.OnGridSquareClicked`
  (params (inGridSquare :type "EMPGridSquare Object Reference"))
  (bind _returnvalue (`self.GetCombatUnitAtCoordinate` (`EMPGridSquare.GridCoordinate` inGridSquare)))
  (if (`KismetSystemLibrary.IsValid` _returnvalue)
    (bind _asbp_base_camp_game_mode (cast `/Game/Framework/BP_BaseCampGameMode` (`GameplayStatics.GetGameMode`)))
    (`EMPBaseCampGameMode.SelectCombatUnit` _asbp_base_camp_game_mode (`EMPCombatUnit.GetCombatUnitData` _returnvalue))))

(event `HandleOnCombatUnitSelected`
  (params (combatUnitData :type "EMPCombatUnitData Object Reference"))
  ;[0.3014 0.7665 1] Combat Unit Events
  (bind _output_get (set `self.SelectedCombatUnit` combatUnitData))
  (`EMPGridSquare.SetSelected` (`self.GetGridSquareAtCoordinate` (`EMPCombatUnitData.GetDesiredLocation` _output_get)) true))

(event `HandleOnSquadSelected`
  (params (squadData :type "EMPSquadData Object Reference"))
  ;[0.941 0.5144 1] Squad Events
  (bind _output_get (set `self.SelectedSquad` squadData))
  (bind _combatunitsinsquad (`EMPSquadData.CombatUnitsInSquad` _output_get))
  (bind _index (`/Game/Framework/Macros_Actor.ForLoopWithDelay_Actor` 0 (- (`KismetArrayLibrary.Array_Length` _combatunitsinsquad) 1) 0.05)
    (:`LoopBody`
      (`self.SpawnCombatUnit` (`|GetArrayItem` _combatunitsinsquad _index)))))

(event `self.OnGridSquareRightClicked`
  (params (inGridSquare :type "EMPGridSquare Object Reference"))
  (bind _selectedcombatunit (`self.SelectedCombatUnit`))
  (if (`KismetSystemLibrary.IsValid` _selectedcombatunit)
    (`EMPSquadManager.MoveCombatUnitToNewDesiredLocation` (subsystem `EMPSquadManager`) _selectedcombatunit (`EMPGridSquare.GridCoordinate` inGridSquare))))

(event `HandleOnSquadDeselected`
  ;[0.941 0.5144 1] Squad Events
  (for _array_element (`self.CombatUnits`)
    (`self.K2_DestroyActor` _array_element))
  (`KismetArrayLibrary.Array_Clear` (`self.CombatUnits`))
  (set `self.SelectedSquad` null))

(event `HandleOnCombatUnitDeselected`
  ;[0.3014 0.7665 1] Combat Unit Events
  (`EMPGridSquare.SetSelected` (`self.GetGridSquareAtCoordinate` (`EMPCombatUnitData.GetDesiredLocation` (`self.SelectedCombatUnit`))) false)
  (set `self.SelectedCombatUnit` null))

(event `self.OnGridSquareHovered`
  (params (inGridSquare :type "EMPGridSquare Object Reference"))
  (`EMPGridSquare.SetHighlighted` inGridSquare true))

(event `self.OnGridSquareUnhovered`
  (params (inGridSquare :type "EMPGridSquare Object Reference"))
  (`EMPGridSquare.SetHighlighted` inGridSquare false))

(event `HandleOnCombatUnitAssignedToSquad`
  (params (unit :type "EMPCombatUnitData Object Reference") (squad :type "EMPSquadData Object Reference"))
  ;[0.3014 0.7665 1] Combat Unit Events
  (if (== squad (`self.SelectedSquad`))
    (`self.SpawnCombatUnit` unit)))

(event `HandleOnCombatUnitMovedToNewDesiredLocation`
  (params (unit :type "EMPCombatUnitData Object Reference") (squad :type "EMPSquadData Object Reference"))
  (bind _returnvalue (`EMPCombatUnitData.GetDesiredLocation` unit))
  (if (== squad (`self.SelectedSquad`))
    (bind _combatunit (`self.GetCombatUnitWithData` unit)
      (:`Found Unit`
        (`EMPGridSquare.SetSelected` (`self.GetGridSquareAtCoordinate` (`EMPCombatUnit.GetGridCoordinate` _combatunit)) false)
        (`EMPCombatUnit.MoveToGridSquare_Timed` _combatunit _returnvalue 0.5)
        (`EMPGridSquare.SetSelected` (`self.GetGridSquareAtCoordinate` _returnvalue) true)))))

(event `HandleOnCombatUnitRemovedFromSquad`
  (params (unit :type "EMPCombatUnitData Object Reference") (squad :type "EMPSquadData Object Reference"))
  ;[0.3014 0.7665 1] Combat Unit Events
  (if (== squad (`self.SelectedSquad`))
    (bind _combatunit (`self.GetCombatUnitWithData` unit)
      (:`Found Unit`
        (`self.K2_DestroyActor` _combatunit)
        (`KismetArrayLibrary.Array_RemoveItem` (`self.CombatUnits`) _combatunit)))))

(event `HandleOnCombatUnitHovered`
  (params (combatUnitData :type "EMPCombatUnitData Object Reference"))
  (bind _output_get (set `self.HoveredCombatUnit` combatUnitData))
  (`EMPGridSquare.SetHighlighted` (`self.GetGridSquareAtCoordinate` (`EMPCombatUnitData.GetDesiredLocation` _output_get)) true))

(event `HandleOnCombatUnitUnhovered`
  (`EMPGridSquare.SetHighlighted` (`self.GetGridSquareAtCoordinate` (`EMPCombatUnitData.GetDesiredLocation` (`self.HoveredCombatUnit`))) false))

(event `SpawnCombatUnit`
  (params (Data :type "EMPCombatUnitData Object Reference"))
  (bind _returnvalue (`|SpawnActorFromClass` (`self.CombatUnitClass`) (`KismetMathLibrary.MakeTransform` (+ (`self.GetWorldLocationFromGridLocation` (`EMPCombatUnitData.GetDesiredLocation` Data)) (0.0 0.0 200.0))) "Undefined" "OverrideRootScale" null null))
  (`self.K2_AttachToActor` _returnvalue self "None" "KeepRelative" "KeepRelative" "KeepRelative" true)
  (set `EMPCombatUnitData.CurrentHealth` (`EMPCombatUnitData.Health` Data) Data)
  (`EMPCombatUnit.SetupCombatUnitMesh` _returnvalue (make `EMPCombatUnitMeshData` true))
  (`KismetArrayLibrary.Array_Add` (`self.CombatUnits`) _returnvalue)
  (`EMPCombatUnit.InitializeCombatUnitData` _returnvalue Data)
  (`EMPCombatUnit.InitializeToGridSquare` _returnvalue (`EMPCombatUnitData.GetDesiredLocation` Data) 0.125))

(fn `UserConstructionScript`)